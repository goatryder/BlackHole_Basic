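; BP_Guard2Test is a guard AI Blueprint that shows its current state as a text emoticon in a WBP_GuardState widget.
; On BeginPlay it casts and caches the widget component's user widget, passes itself as the guard reference, and displays the initial GuardState.
; OnStateChanged calls UpdateStateWidget, which maps each state, from idle and patrolling to alerted and chasing, to an emoticon via a Select node.
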(event `self.ReceiveBeginPlay`
  (bind _aswbp_guard_state (cast `/Game/UI/WBP_GuardState` (`WidgetComponent.GetUserWidgetObject` (`self.Widget`))))
  (bind _output_get (set `self.WidgetStatesRef` _aswbp_guard_state))
  (set `/Game/UI/WBP_GuardState.Guard_REF` self _output_get)
  (`self.Update State Widget` (`self.GuardState`)))

(event `self.OnStateChanged`
  (params (NewState :type "EAIState Enum" :default "Idle"))
  (`self.Update State Widget` NewState))

(fn `Update State Widget`
  (params (`AI State` :type "EAIState Enum" :default "Idle"))
  (bind _widgetstatesref (`self.WidgetStatesRef`))
  (`/Engine/EditorBlueprintResources/StandardMacros.IsValid` _widgetstatesref
    (:`Is Valid`
      (`/Game/UI/WBP_GuardState.UpdateText` _widgetstatesref (select `EAIState` `AI State` :`Idle` ":)" :`Suspicious` "?" :`Alerted` "!" :`Patrolling` "-_-" :`ChassingTarget` ">:c" :`MovingBackToGuardPoint` ":(" :`LooseChassingTarget` "!?" :!type "Text")))))

(fn `UserConstructionScript`)